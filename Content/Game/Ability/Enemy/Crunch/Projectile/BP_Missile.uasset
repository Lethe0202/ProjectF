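; BP_Missile is the missile projectile for the enemy Crunch's abilities.
; A sphere overlap with an actor hostile to its owning PFCharacterBase, or any hit event, calls CallOnProjectileEffect with the target and hit result, then destroys the missile.
; Destruction spawns a scaled-down rocket explosion emitter and sound at the mesh location.
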(event OnComponentBeginOverlap(Sphere)
  (params (OverlappedComponent :type Primitive%20Component%20Object%20Reference) (OtherActor :type Actor%20Object%20Reference) (OtherComp :type Primitive%20Component%20Object%20Reference) (OtherBodyIndex :type Integer) (bFromSweep :type Boolean) (SweepResult :type Hit%20Result%20Structure%20%28by%20ref%29))
  (bind _aspfcharacter_base (Utilities|Casting|CastToPFCharacterBase (Components|GetOwner)))
  (if (Utilities|Enum|Equal(Enum) (Class|PFCharacterBase|GetTeamAttitudeTowardsBP _aspfcharacter_base OtherActor) "Hostile")
    (Default|CallOnProjectileEffect self OtherActor SweepResult)
    (Actor|DestroyActor)))

(event EventBeginPlay)

(event Collision|EventActorBeginOverlap
  (params (OtherActor :type Actor%20Object%20Reference)))

(event EventTick
  (params (DeltaSeconds :type Float%20%28single-precision%29)))

(event EventDestroyed
  (bind _staticmesh (Variables|Default|GetStaticMesh))
  (bind _returnvalue (Transformation|GetWorldLocation _staticmesh))
  (Effects|SpawnEmitteratLocation "/Game/Art/MilitaryWeapSilver/FX/P_RocketLauncher_Explosion_01.P_RocketLauncher_Explosion_01" _returnvalue "0, 0, 0" "0.100000,0.100000,0.100000")
  (Audio|SpawnSoundatLocation "/Game/Art/MilitaryWeapSilver/Sound/RocketLauncher/Cues/RocketLauncher_Explosion_Cue.RocketLauncher_Explosion_Cue" _returnvalue "0, 0, 0" 1.0 1.0 0.0 0 0))

(event Collision|EventHit
  (params (MyComp :type Primitive%20Component%20Object%20Reference) (Other :type Actor%20Object%20Reference) (OtherComp :type Primitive%20Component%20Object%20Reference) (bSelfMoved :type Boolean) (HitLocation :type Vector :default "0, 0, 0") (HitNormal :type Vector :default "0, 0, 0") (NormalImpulse :type Vector :default "0, 0, 0") (Hit :type Hit%20Result%20Structure%20%28by%20ref%29))
  (Default|CallOnProjectileEffect self Other Hit)
  (Actor|DestroyActor))

(fn ConstructionScript)