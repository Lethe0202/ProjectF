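; BP_IntroSequence plays a first-time intro level sequence when the game starts with no save file.
; On BeginPlay it checks the PFGameInstance save manager, locks input to UI and shows a black screen widget at once.
; After a one-second delay it hides the HUD, removes the black screen and plays the sequence with the player pawn bound by tag.
; When the sequence finishes, it restores the HUD and game-only input.
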(event Custom|HandleFinished
  (bind _returnvalue (Game|GetPlayerController 0))
  (bind _aspfplayer_controller (Utilities|Casting|CastToPFPlayerController _returnvalue))
  (Class|PFPlayerController|VisibleHUD _aspfplayer_controller true)
  (Input|SetInputModeGameOnly _returnvalue false))

(event EventBeginPlay
  (bind _returnvalue (Game|GetPlayerController 0))
  (bind _level_sequence (Variables|Default|GetLevel%20Sequence))
  (bind _aspfgame_instance (Utilities|Casting|CastToPFGameInstance (Game|GetGameInstance)))
  (bind _returnvalue_2 (Class|PFGameInstance|GetSaveManager _aspfgame_instance))
  (if (not (Class|SaveManager|IsHaveSaveFile _returnvalue_2))
    (Input|SetInputModeUIOnly (Game|GetPlayerController 0) 0 "LockInFullscreen" true)
    (Utilities|FlowControl|Sequence
      (:then_0
        (bind _returnvalue_3 (UserInterface|CreateWidget "/Game/Game/UI/HUD/WBP_BlackScreen.WBP_BlackScreen_C" _returnvalue))
        (UserInterface|Viewport|AddtoViewport _returnvalue_3 10))
      (:then_1
        (Utilities|FlowControl|Delay 1.0)
        (bind _aspfplayer_controller (Utilities|Casting|CastToPFPlayerController _returnvalue))
        (Class|PFPlayerController|VisibleHUD _aspfplayer_controller false)
        (Widget|RemovefromParent _returnvalue_3))
      (:then_2
        (Utilities|FlowControl|Delay 1.0)
        (bind (_outactor _returnvalue_4) (Sequencer|Player|CreateLevelSequencePlayer _level_sequence))
        (EventDispatchers|BindEventtoOnFinished _returnvalue_4 (delegate Custom|HandleFinished))
        (Class|LevelSequenceActor|SetBinding _outactor (Class|MovieSceneSequence|FindBindingbyTag _level_sequence "Player") (Utilities|Array|MakeArray (Game|Player|GetPlayerPawn 0)) false)
        (Sequencer|Player|Play _returnvalue_4 :!class /Script/MovieScene.MovieSceneSequencePlayer)))))

(event Collision|EventActorBeginOverlap
  (params (OtherActor :type Actor%20Object%20Reference)))

(event EventTick
  (params (DeltaSeconds :type Float%20%28single-precision%29)))

(fn ConstructionScript)