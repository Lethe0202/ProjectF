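; Base Blueprint for boss enemies, handling the overhead status widget and the death cinematic.
; Health and stamina component delegates feed the progress bars in the WBP_EnemyStatus widget.
; Unpossession during gameplay serves as the death trigger, hiding the widget and playing DeadSequence with HUD hidden and UI-only input, both restored when it finishes.
; Tick writes the combat state into a text render hidden at BeginPlay, apparently for debugging.
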(event Custom|OnStaminaChanged_이벤트
  (params (OldValue :type Float%20%28single-precision%29) (NewValue :type Float%20%28single-precision%29) (MaxValue :type Float%20%28single-precision%29) (Instigator :type Actor%20Object%20Reference))
  (bind _aswbp_enemy_status (Utilities|Casting|CastToWBP_EnemyStatus (UserInterface|GetWidget (Variables|Default|GetHealthWidgetComponent))))
  (Class|ProgressHUDWidget|OnProgressChanged (Variables|/Game/Game/UI/HUD/Combat/WBP_EnemyStatus.WBP_EnemyStatus_C|GetWBP_StaminaBar _aswbp_enemy_status) OldValue NewValue MaxValue Instigator))

(event Custom|커스텀이벤트
  (params (OldValue :type Float%20%28single-precision%29) (NewValue :type Float%20%28single-precision%29) (MaxValue :type Float%20%28single-precision%29) (Instigator :type Actor%20Object%20Reference))
  (bind _aswbp_enemy_status (Utilities|Casting|CastToWBP_EnemyStatus (UserInterface|GetWidget (Variables|Default|GetHealthWidgetComponent))))
  (Class|ProgressHUDWidget|OnProgressChanged (Variables|/Game/Game/UI/HUD/Combat/WBP_EnemyStatus.WBP_EnemyStatus_C|GetWBP_HealthBar _aswbp_enemy_status) OldValue NewValue MaxValue Instigator))

(event Custom|OnFinish
  (bind _returnvalue (Game|GetPlayerController 0))
  (bind _aspfplayer_controller (Utilities|Casting|CastToPFPlayerController _returnvalue))
  (Class|PFPlayerController|VisibleHUD _aspfplayer_controller true)
  (Input|SetInputModeGameOnly _returnvalue false))

(event EventBeginPlay
  (Rendering|SetVisibility (Variables|Default|GetTextRender) false false)
  (Utilities|FlowControl|Sequence
    (:then_0
      (EventDispatchers|BindEventtoOnHealthStatusChanged (Variables|Default|GetHealthComponent) (delegate Custom|커스텀이벤트)))
    (:then_1
      (EventDispatchers|AssignOnStaminaChanged (Variables|Default|GetStaminaComponent) (delegate Custom|OnStaminaChanged_이벤트)))))

(event EventUnpossessed
  (params (OldController :type Controller%20Object%20Reference))
  (bind _returnvalue (Game|GetPlayerController 0))
  (bind _deadsequence (Variables|Default|GetDeadSequence))
  (bind _returnvalue_2 (Class|PFFunctionLibrary|GetActorWorld self))
  (bind _returnvalue_3 (Class|PFFunctionLibrary|IsinGame _returnvalue_2))
  (if _returnvalue_3
    (Utilities|FlowControl|Sequence
      (:then_0
        (Development|SetHiddeninGame (Variables|Default|GetHealthWidgetComponent) true true))
      (:then_1
        (if (Utilities|IsValid _deadsequence)
          (bind _returnvalue_4 (Sequencer|Player|CreateLevelSequencePlayer _deadsequence))
          (EventDispatchers|BindEventtoOnFinished _returnvalue_4 (delegate Custom|OnFinish))
          (Sequencer|Player|Play _returnvalue_4 :!class /Script/MovieScene.MovieSceneSequencePlayer)
          (bind _aspfplayer_controller (Utilities|Casting|CastToPFPlayerController _returnvalue))
          (Class|PFPlayerController|VisibleHUD _aspfplayer_controller false)
          (Input|SetInputModeUIOnly _returnvalue 0 "LockInFullscreen" true))))))

(event EventTick
  (params (DeltaSeconds :type Float%20%28single-precision%29))
  (bind _returnvalue (Class|CombatStateComponent|GetCurrentState (Variables|Default|GetCombatStateComponent)))
  (Rendering|Components|TextRender|SetText (Variables|Default|GetTextRender) (Utilities|Text|ToText(String) (Utilities|String|EnumtoString _returnvalue))))

(fn ConstructionScript)