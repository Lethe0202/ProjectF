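; Base enemy Blueprint that links health, stamina and combat state to the enemy's status display.
; On BeginPlay it subscribes to health and stamina change events, forwarding values to the progress bars in the WBP_EnemyStatus widget component.
; Tick writes the current combat state to a text render, which BeginPlay hides, likely as a debug readout.
; When unpossessed, it hides the status widget.
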(event Custom|OnStaminaChanged_이벤트
  (params (OldValue :type Float%20%28single-precision%29) (NewValue :type Float%20%28single-precision%29) (MaxValue :type Float%20%28single-precision%29) (Instigator :type Actor%20Object%20Reference))
  (bind _aswbp_enemy_status (Utilities|Casting|CastToWBP_EnemyStatus (UserInterface|GetWidget (Variables|Default|GetHealthWidgetComponent))))
  (Class|ProgressHUDWidget|OnProgressChanged (Variables|/Game/Game/UI/HUD/Combat/WBP_EnemyStatus.WBP_EnemyStatus_C|GetWBP_StaminaBar _aswbp_enemy_status) OldValue NewValue MaxValue Instigator))

(event Custom|커스텀이벤트
  (params (OldValue :type Float%20%28single-precision%29) (NewValue :type Float%20%28single-precision%29) (MaxValue :type Float%20%28single-precision%29) (Instigator :type Actor%20Object%20Reference))
  (bind _aswbp_enemy_status (Utilities|Casting|CastToWBP_EnemyStatus (UserInterface|GetWidget (Variables|Default|GetHealthWidgetComponent))))
  (Class|ProgressHUDWidget|OnProgressChanged (Variables|/Game/Game/UI/HUD/Combat/WBP_EnemyStatus.WBP_EnemyStatus_C|GetWBP_HealthBar _aswbp_enemy_status) OldValue NewValue MaxValue Instigator))

(event EventBeginPlay
  (Rendering|SetVisibility (Variables|Default|GetTextRender) false false)
  (Utilities|FlowControl|Sequence
    (:then_0
      (EventDispatchers|BindEventtoOnHealthStatusChanged (Variables|Default|GetHealthComponent) (delegate Custom|커스텀이벤트)))
    (:then_1
      (EventDispatchers|AssignOnStaminaChanged (Variables|Default|GetStaminaComponent) (delegate Custom|OnStaminaChanged_이벤트)))))

(event EventUnpossessed
  (params (OldController :type Controller%20Object%20Reference))
  (Development|SetHiddeninGame (Variables|Default|GetHealthWidgetComponent) true true))

(event EventTick
  (params (DeltaSeconds :type Float%20%28single-precision%29))
  (bind _returnvalue (Class|CombatStateComponent|GetCurrentState (Variables|Default|GetCombatStateComponent)))
  (Rendering|Components|TextRender|SetText (Variables|Default|GetTextRender) (Utilities|Text|ToText(String) (Utilities|String|EnumtoString _returnvalue))))

(fn ConstructionScript)