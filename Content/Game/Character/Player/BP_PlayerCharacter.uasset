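; Player character Blueprint with dynamic combat cameras, screen effects and a hidden combat-state debug text.
; Camera modes reattach FollowCamera to Near or Counter booms, and ClearCamera manages eased moves back, restoring targeting on completion.
; Z triggers a physics-blended hit reaction with an impulse, while ScreenShatter captures the scene, then spawns break actor and glass widget.
; Ladder climbing, marked unused, alternates montages, lerps height per rung and feeds hand offsets to ABP_Player.
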(event Custom|ClearCamera
  (bind _cachecameratransform (Variables|Default|GetCacheCameraTransform))
  (bind (_location _rotation) (Math|Transform|BreakTransform _cachecameratransform))
  (Utilities|FlowControl|Sequence
    (:then_0
      ;[0.15 0.15 0.15 0.5] Default
      (Components|MoveComponentTo (Variables|Default|GetFollowCamera) _location _rotation true true 0.4 true) ; enters at Stop
    )))

(event Custom|커스텀이벤트
  (CameraShakes|StartCameraShake (Variables|Default|GetCameraShakeSource) (stale Custom|StartCameraShake CameraShakeClass) 1.0 "CameraLocal" "0, 0, 0"))

(event Custom|StartCameraShake
  (params (CameraShakeClass :type Camera%20Shake%20Base%20Class%20Reference))
  (Utilities|Time|SetTimerbyEvent (delegate Custom|커스텀이벤트) (Utilities|Time|GetWorldDeltaSeconds)))

(event Input|EnhancedActionEvents|EnhancedInputActionIA_Move
  (params (ActionValue :type Vector%202D%20Structure) (ElapsedSeconds :type Float%20%28double-precision%29) (TriggeredSeconds :type Float%20%28double-precision%29) (InputAction :type Input%20Action%20Object%20Reference :default "/Game/Game/Character/Player/Input/Actions/IA_Move.IA_Move"))
  (bind _mesh (Variables|Character|GetMesh))
  ;[1 0 0 0.5 36] Ladder not use
  (:Started
    (if (Utilities|Enum|Equal(Enum) (Variables|/Script/Engine.CharacterMovementComponent|GetMovementMode (Variables|Character|GetCharacterMovement)) "MOVE_Flying")
      (if (not (Audio|Components|Audio|IsPlaying (Variables|Default|Get타임라인)))
        (Variables|Default|SetCurZ (Transformation|GetActorLocation))
        (if (>= (Utilities|Array|Length (Variables|Default|GetLadder%20Bar%20Height%20Array)) (+ (Variables|Default|GetPelvisOffset) 2))
          (Utilities|FlowControl|FlipFlop
            (:A
              (Animation|Montage|PlayMontage _mesh "/Game/Art/Animation/Golem/Ladder/anim_Ladder2_Montage.anim_Ladder2_Montage"
                (:then
                  (Utilities|FlowControl|Sequence
                    (:then_0
                      (bind _새_트랙_0 (Timeline|타임라인 PlayFromStart)
                        (:Update
                          (Transformation|SetActorLocation (Math|Vector|MakeVector (.x (Variables|Default|GetCurZ)) (.y (Variables|Default|GetCurZ)) (Math|Float|Lerp (.z (Variables|Default|GetCurZ)) (Utilities|Array|Get(acopy) (Variables|Default|GetLadder%20Bar%20Height%20Array) (Variables|Default|GetPelvisOffset)) _새_트랙_0)) false false))
                        (:Finished
                          (Variables|Default|SetPelvisOffset (+ (Variables|Default|GetPelvisOffset) 1))
                          (Variables|Default|SetCurZ (Transformation|GetActorLocation)))))
                    (:then_1
                      (bind _output_get (Variables|Ladder|Sethand_r_ZLocation (- (Utilities|Array|Get(acopy) (Variables|Default|GetLadder%20Bar%20Height%20Array) (+ (Variables|Default|GetPelvisOffset) 2)) (.z (Transformation|GetSocketLocation (Variables|Character|GetMesh) "hand_r")))))
                      (bind _asabp_player (Utilities|Casting|CastToABP_Player (Components|SkeletalMesh|GetAnimInstance (Variables|Character|GetMesh))))
                      (Variables|/Game/Game/Character/Player/Animation/ABP_Player.ABP_Player_C|SetRightHandHeight _asabp_player _output_get)
                      (Variables|/Game/Game/Character/Player/Animation/ABP_Player.ABP_Player_C|SetLeftHandHeight _asabp_player (- (Utilities|Array|Get(acopy) (Variables|Default|GetLadder%20Bar%20Height%20Array) (+ (Variables|Default|GetPelvisOffset) 1)) (.z (Transformation|GetSocketLocation (Variables|Character|GetMesh) "hand_l")))))))))
            (:B
              (Animation|Montage|PlayMontage _mesh "/Game/Art/Animation/Golem/Ladder/anim_Ladder1_Montage.anim_Ladder1_Montage"
                (:then
                  (Utilities|FlowControl|Sequence
                    (:then_0
                      (Timeline|타임라인 PlayFromStart))
                    (:then_1
                      (bind _output_get_2 (Variables|Ladder|Sethand_l_ZLocation (- (Utilities|Array|Get(acopy) (Variables|Default|GetLadder%20Bar%20Height%20Array) (+ (Variables|Default|GetPelvisOffset) 2)) (.z (Transformation|GetSocketLocation (Variables|Character|GetMesh) "hand_l")))))
                      (bind _asabp_player_2 (Utilities|Casting|CastToABP_Player (Components|SkeletalMesh|GetAnimInstance (Variables|Character|GetMesh))))
                      (Variables|/Game/Game/Character/Player/Animation/ABP_Player.ABP_Player_C|SetLeftHandHeight _asabp_player_2 _output_get_2)
                      (Variables|/Game/Game/Character/Player/Animation/ABP_Player.ABP_Player_C|SetRightHandHeight _asabp_player_2 (- (Utilities|Array|Get(acopy) (Variables|Default|GetLadder%20Bar%20Height%20Array) (+ (Variables|Default|GetPelvisOffset) 1)) (.z (Transformation|GetSocketLocation (Variables|Character|GetMesh) "hand_r"))))))))))
          (else
            (Animation|Montage|PlayMontage 0 "/Game/Art/Animation/Golem/Ladder/anim_ClimbUp_At_Top_Montage.anim_ClimbUp_At_Top_Montage")))))))

(event EventBeginPlay
  (Rendering|SetVisibility (Variables|Default|GetTextRender) false false))

(event Collision|EventActorBeginOverlap
  (params (OtherActor :type Actor%20Object%20Reference)))

(event EventTick
  (params (DeltaSeconds :type Float%20%28single-precision%29))
  (bind _returnvalue (Class|CombatStateComponent|GetCurrentState (Variables|Default|GetCombatStateComponent)))
  (Rendering|Components|TextRender|SetText (Variables|Default|GetTextRender) (Utilities|Text|ToText(String) (Utilities|String|EnumtoString _returnvalue))))

(event EventChangeCameraMode
  (params (DynamicCameraType :type EDynamicCameraType%20Enum :default "Default"))
  (Utilities|FlowControl|Sequence
    (:then_1
      (switch Utilities|FlowControl|Switch|SwitchonEDynamicCameraType DynamicCameraType
        (:Default
          ;[0.15 0.15 0.15 0.5] Default
          (CallFunction|ChangeDefaultCamera)
          (Components|MoveComponentTo (Variables|Default|GetFollowCamera) (.Location (Math|Transform|BreakTransform (Variables|Default|GetCacheCameraTransform))) (.Rotation (Math|Transform|BreakTransform (Variables|Default|GetCacheCameraTransform))) true true 0.4 true)
          (Variables|Default|SetbUpdateTargeting true))
        (:Near
          (Variables|Default|SetbUpdateTargeting false)
          (Variables|Default|SetCacheCameraTransform (Transformation|GetRelativeTransform (Variables|Default|GetFollowCamera)))
          (Utilities|FlowControl|Sequence
            (:then_0
              ;[0.15 0.15 0.15 0.5] Near
              (CallFunction|ClearCamera))
            (:then_1
              (Transformation|SetRelativeRotation (Variables|Default|GetNear_CameraBoom) (Math|Rotator|MakeRotator 0.0 0.0 (- (.Yaw (Math|Rotator|BreakRotator (Transformation|GetActorRotation))) 6e+01)) false false)
              (Transformation|AttachComponentToComponent (Variables|Default|GetFollowCamera) (Variables|Default|GetNear_CameraBoom) "None" "KeepRelative" "KeepRelative" "KeepRelative" true))))
        (:Face
          (Variables|Default|SetbUpdateTargeting false)
          (Variables|Default|SetCacheCameraTransform (Transformation|GetRelativeTransform (Variables|Default|GetFollowCamera)))
          ;[0.15 0.15 0.15 0.5] Face
          (Utilities|FlowControl|Sequence
            (:then_0
              (CallFunction|ClearCamera))
            (:then_1
              (Transformation|SetRelativeRotation (Variables|Default|GetNear_CameraBoom) (Math|Rotator|MakeRotator 0.0 0.0 (- (.Yaw (Math|Rotator|BreakRotator (Transformation|GetActorRotation))) 1.2e+02)) false false)
              (Transformation|AttachComponentToComponent (Variables|Default|GetFollowCamera) (Variables|Default|GetNear_CameraBoom) "None" "KeepRelative" "KeepRelative" "KeepRelative" true))))
        (:Counter
          (Utilities|FlowControl|Sequence
            (:then_0
              (CallFunction|ClearCamera)
              (Transformation|SetRelativeTransform (Variables|Default|GetFollowCamera) (Math|Transform|MakeTransform "0, 0, 0") false false))
            (:then_1
              (Transformation|SetRelativeRotation (Variables|Default|GetCounter_CameraBoom) (Math|Rotator|MakeRotator 0.0 0.0 (- (.Yaw (Math|Rotator|BreakRotator (Transformation|GetActorRotation))) 3e+01)) false false)
              (Transformation|AttachComponentToComponent (Variables|Default|GetFollowCamera) (Variables|Default|GetCounter_CameraBoom) "None" "KeepRelative" "KeepRelative" "KeepRelative" true))))))))

(event Input|KeyboardEvents|Z
  (params (Key :type Key%20Structure :default "None"))
  (bind _mesh (Variables|Character|GetMesh))
  (bind _in_bone_name (Variables|Default|GetIn%20Bone%20Name))
  ;[0.15 0.15 0.15 0.5] 코멘트
  (:Pressed
    (Utilities|FlowControl|Sequence
      (:then_0
        (bind _새_트랙_0 (Timeline|타임라인_0 PlayFromStart)
          (:Update
            (Variables|Default|SetPhysics%20Blend%20Weight _새_트랙_0)
            (Class|SkeletalMeshComponent|SetAllBodiesBelowPhysicsBlendWeight _mesh _in_bone_name (Variables|Default|GetPhysics%20Blend%20Weight) false true))
          (:Finished
            (Class|SkeletalMeshComponent|SetAllBodiesPhysicsBlendWeight _mesh 0.0 false)
            (Class|SkeletalMeshComponent|SetAllBodiesSimulatePhysics (Variables|Character|GetMesh) false))))
      (:then_1
        (Class|SkeletalMeshComponent|SetAllBodiesBelowSimulatePhysics _mesh _in_bone_name true true)
        (Utilities|FlowControl|Delay 0.01)
        (Physics|AddImpulse _mesh (* (Transformation|GetActorForwardVector (Game|GetPlayerCharacter 0)) 1e+04) (Variables|Default|GetIn%20Bone%20Name) true)))))

(fn ConstructionScript)

(fn ChangeDefaultCamera
  (bind _returnvalue (Transformation|AttachComponentToComponent (Variables|Default|GetFollowCamera) (Variables|Default|GetCameraBoom) "None" "KeepWorld" "KeepWorld" "KeepWorld" true))
  (if _returnvalue
    _))

(fn TestStartLadder
  (params (Ladder :type BP%20Procedural%20Ladder%20Object%20Reference))
  (bind _returnvalue (Transformation|GetActorLocation))
  (Utilities|FlowControl|Sequence
    (:then_0
      (Pawn|Components|CharacterMovement|SetMovementMode (Variables|Character|GetCharacterMovement) "MOVE_Flying" 0)
      (Variables|Default|SetPelvisOffset 1)
      (bind _output_get (Variables|Default|SetLadder%20Bar%20Height%20Array (Variables|/Game/Game/Utility/BP_ProceduralLadder.BP_ProceduralLadder_C|GetLadderBarHeightArray Ladder)))
      (Transformation|SetActorLocation (Math|Vector|MakeVector (.x _returnvalue) (.y _returnvalue) (Utilities|Array|Get(acopy) _output_get 1)) false false)
      (Animation|Montage|MontagePlay (Components|SkeletalMesh|GetAnimInstance (Variables|Character|GetMesh)) "/Game/Art/Animation/Golem/Ladder/anim_Ladder1_Montage.anim_Ladder1_Montage" 1.0 "MontageLength" 0.0 true))
    (:then_1
      (Variables|Ladder|Sethand_l_ZLocation (- (- (Utilities|Array|Get(acopy) (Variables|Default|GetLadder%20Bar%20Height%20Array) (+ (Variables|Default|GetPelvisOffset) 2)) (.z (Transformation|GetSocketLocation (Variables|Character|GetMesh) "hand_l"))) 5e+01))
      (Variables|Ladder|Sethand_r_ZLocation (- (- (Utilities|Array|Get(acopy) (Variables|Default|GetLadder%20Bar%20Height%20Array) (+ (Variables|Default|GetPelvisOffset) 2)) (.z (Transformation|GetSocketLocation (Variables|Character|GetMesh) "hand_r"))) 6e+01))
      (bind _asabp_player (Utilities|Casting|CastToABP_Player (Components|SkeletalMesh|GetAnimInstance (Variables|Character|GetMesh))))
      (Variables|/Game/Game/Character/Player/Animation/ABP_Player.ABP_Player_C|SetOnLadder _asabp_player true)
      (Variables|/Game/Game/Character/Player/Animation/ABP_Player.ABP_Player_C|SetLeftHandOffsetTarget _asabp_player (Variables|Ladder|Gethand_l_ZLocation))
      (Variables|/Game/Game/Character/Player/Animation/ABP_Player.ABP_Player_C|SetRightHandOffsetTarget _asabp_player (Variables|Ladder|Gethand_r_ZLocation)))))

(fn ScreenShatter
  (Rendering|SceneCapture|CaptureScene (Variables|Default|GetSceneCaptureComponent2D) :!class /Script/Engine.SceneCaptureComponent2D)
  (Game|SpawnActorfromClass "/Game/Game/Utility/ScreenBreak/BP_Screenbreak.BP_Screenbreak_C" (Math|Transform|MakeTransform "0.000000,0.000000,400.000000") "Undefined" "MultiplyWithRoot" 0 0)
  (bind _returnvalue (UserInterface|CreateWidget "/Game/Game/Utility/ScreenBreak/W_GlassBreak.W_GlassBreak_C"))
  (UserInterface|Viewport|AddtoViewport _returnvalue 1))