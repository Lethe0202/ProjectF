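; Player parkour component that picks and plays a traversal montage on its owning Character.
; StartParkour casts the target to BP_ParkourSpline and uses FindEndPoint to get the spline's start and end locations.
; The absolute height gap to the spline start selects a ledge climb or, when small, a mantle or hurdle by distance to the spline end.
; Gaps outside those two height bands play nothing, and BeginPlay and Tick are empty.
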(event EventBeginPlay)

(event EventTick
  (params (DeltaSeconds :type Float%20%28single-precision%29)))

(fn StartParkour
  (params (TargetActor :type Actor%20Object%20Reference))
  (bind _returnvalue (Components|GetOwner))
  (bind _parkourdata (LocalVariables|GetParkourData))
  (bind _startsplinelocation (Utilities|Struct|BreakS_ParkourData _parkourdata))
  (bind _returnvalue_2 (Transformation|GetActorLocation _returnvalue))
  (bind _returnvalue_3 (- (.z _startsplinelocation) (.z _returnvalue_2)))
  (bind _returnvalue_4 (Math|Float|Absolute(Float) _returnvalue_3))
  (bind _asbp_parkour_spline (Utilities|Casting|CastToBP_ParkourSpline TargetActor))
  (Default|FindEndPoint _asbp_parkour_spline TargetActor (LocalVariables|GetParkourData))
  (bind _as캐릭터 (Utilities|Casting|CastToCharacter (Components|GetOwner)))
  (if (and (> _returnvalue_4 5e+01) (< _returnvalue_4 9e+01))
    (Animation|PlayAnimMontage _as캐릭터 "/Game/Art/Animation/Player_Gideon/Action/Parkour/ClimbUpTheLedgeUE5_Montage.ClimbUpTheLedgeUE5_Montage" 1.0 "None")
    (elif (and (> _returnvalue_4 0.0) (< _returnvalue_4 2e+01))
      (if (> (Math|Vector|Distance(Vector) (.EndSplineLocation (Utilities|Struct|BreakS_ParkourData (LocalVariables|GetParkourData))) (Transformation|GetActorLocation (Components|GetOwner))) 1.5e+02)
        (Animation|PlayAnimMontage _as캐릭터 "/Game/Art/Animation/Player_Gideon/Action/Parkour/anim_Mantle_1M_R_Montage.anim_Mantle_1M_R_Montage" 1.0 "None")
        (return "")
        (else
          (Animation|PlayAnimMontage _as캐릭터 "/Game/Art/Animation/Player_Gideon/Action/Parkour/M_Neutral_Traversal_Hurdle_1_0_stand_F_V2_Lfoot3_Montage.M_Neutral_Traversal_Hurdle_1_0_stand_F_V2_Lfoot3_Montage" 1.0 "None")
          (return ""))))))