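; Player combat component that plays a counterattack against a target.
; PlayCounterEffect waits briefly, sets invincibility and plays a back-dash montage, then a sword combo montage on blend out.
; As the combo starts, global time dilation drops sharply while the owner's custom dilation compensates.
; Tick uses real time to lerp the owner horizontally to just short of the target over one second, then restores both dilations.
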(event Custom|OnMontageEnded_이벤트
  (params (Montage :type Anim%20Montage%20Object%20Reference) (bInterrupted :type Boolean))
  (bind _returnvalue (Components|GetOwner))
  (Class|CombatStateComponent|SetInvincible true)
  (Animation|Montage|PlayMontage (Variables|/Script/Engine.Character|GetMesh (stale EventPlayCounterEffect _as캐릭터)) "/Game/Art/Animation/Player_Gideon/Locomotion/Action/10_Frank_ActionRPG_Sword_Back_Dash_Montage.10_Frank_ActionRPG_Sword_Back_Dash_Montage"
    (:OnBlendOut
      (Animation|Montage|PlayMontage (Variables|/Script/Engine.Character|GetMesh (stale EventPlayCounterEffect _as캐릭터)) "/Game/Art/Animation/Player_Gideon/Locomotion/Action/51_Frank_ActionRPG_Sword_Combo_A5_Montage.51_Frank_ActionRPG_Sword_Combo_A5_Montage"
        (:then
          (Variables|Default|SetStart true)
          (Variables|Default|SetStartTime (Utilities|Time|GetRealTimeSeconds))
          (Variables|Default|SetStartLocation (Transformation|GetActorLocation (Components|GetOwner)))
          (Utilities|FlowControl|Sequence
            (:then_1
              ;[0.15 0.15 0.15 0.5] 도지 시작할때 빠르게
              (Utilities|Time|SetGlobalTimeDilation 0.01)
              (Variables|/Script/Engine.Actor|SetCustomTimeDilation _returnvalue 1e+02)
              ;[0.15 0.15 0.15 0.5] 시작 이후 잠깐동안 느리게
              (Utilities|FlowControl|Delay 0.01)
              (Variables|/Script/Engine.Actor|SetCustomTimeDilation _returnvalue 5e+01))))))))

(event EventBeginPlay)

(event EventTick
  (params (DeltaSeconds :type Float%20%28single-precision%29))
  (bind _startlocation (Variables|Default|GetStartLocation))
  (bind (_x _y _z) (Math|Vector|BreakVector _startlocation))
  (if (Variables|Default|GetStart)
    (Utilities|FlowControl|Sequence
      (:then_0
        (bind _output_get (Variables|Default|SetElapedTime (- (Utilities|Time|GetRealTimeSeconds) (Variables|Default|GetStartTime))))
        (Variables|Default|SetAlpha (/ _output_get 1.0)))
      (:then_1
        (if (Utilities|IsValid (stale EventPlayCounterEffect Target))
          (Transformation|SetActorLocation (Components|GetOwner) (Math|Vector|MakeVector (.X (Math|Vector|BreakVector (Math|Vector|Lerp(Vector) (Math|Vector|MakeVector _x _y 0.0) (- (Transformation|GetActorLocation (stale EventPlayCounterEffect Target)) (* (Math|Vector|Normalize (- (Transformation|GetActorLocation (stale EventPlayCounterEffect Target)) (Variables|Default|GetStartLocation))) 1e+02)) (Variables|Default|GetAlpha)))) (.Y (Math|Vector|BreakVector (Math|Vector|Lerp(Vector) (Math|Vector|MakeVector _x _y 0.0) (- (Transformation|GetActorLocation (stale EventPlayCounterEffect Target)) (* (Math|Vector|Normalize (- (Transformation|GetActorLocation (stale EventPlayCounterEffect Target)) (Variables|Default|GetStartLocation))) 1e+02)) (Variables|Default|GetAlpha)))) _z) false false)))
      (:then_2
        (if (>= (Variables|Default|GetAlpha) 1.0)
          (Variables|Default|SetStart false)
          (Variables|Default|SetElapedTime 0.0)
          (Variables|Default|SetAlpha 0.0)
          ;[0.15 0.15 0.15 0.5] 원래대로
          (Utilities|Time|SetGlobalTimeDilation 1.0)
          (Variables|/Script/Engine.Actor|SetCustomTimeDilation (Components|GetOwner) 1.0))))))

(event EventPlayCounterEffect
  (params (Target :type Actor%20Object%20Reference))
  (bind _returnvalue (Components|GetOwner))
  (bind _as캐릭터 (Utilities|Casting|CastToCharacter _returnvalue))
  (Utilities|FlowControl|Delay 0.2)
  (Class|CombatStateComponent|SetInvincible true)
  (Animation|Montage|PlayMontage (Variables|/Script/Engine.Character|GetMesh _as캐릭터) "/Game/Art/Animation/Player_Gideon/Locomotion/Action/10_Frank_ActionRPG_Sword_Back_Dash_Montage.10_Frank_ActionRPG_Sword_Back_Dash_Montage"
    (:OnBlendOut
      (Animation|Montage|PlayMontage (Variables|/Script/Engine.Character|GetMesh _as캐릭터) "/Game/Art/Animation/Player_Gideon/Locomotion/Action/51_Frank_ActionRPG_Sword_Combo_A5_Montage.51_Frank_ActionRPG_Sword_Combo_A5_Montage"
        (:then
          (Variables|Default|SetStart true)
          (Variables|Default|SetStartTime (Utilities|Time|GetRealTimeSeconds))
          (Variables|Default|SetStartLocation (Transformation|GetActorLocation (Components|GetOwner)))
          (Utilities|FlowControl|Sequence
            (:then_1
              ;[0.15 0.15 0.15 0.5] 도지 시작할때 빠르게
              (Utilities|Time|SetGlobalTimeDilation 0.01)
              (Variables|/Script/Engine.Actor|SetCustomTimeDilation _returnvalue 1e+02)
              ;[0.15 0.15 0.15 0.5] 시작 이후 잠깐동안 느리게
              (Utilities|FlowControl|Delay 0.01)
              (Variables|/Script/Engine.Actor|SetCustomTimeDilation _returnvalue 5e+01))))))))