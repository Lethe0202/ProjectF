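; BP_Screenbreak is a short-lived actor that shatters a Geometry Collection, apparently as a screen-break effect.
; On BeginPlay it enables collision damage, fires a radial velocity impulse from just along the collection's forward axis, then turns on gravity.
; Impulse strength scales by the inverse of global time dilation to compensate for slowed or sped-up time.
; The actor destroys itself after a brief delay.
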(event EventBeginPlay
  (bind _geometrycollection (Variables|Default|GetGeometryCollection))
  (Class|GeometryCollectionComponent|SetEnableDamagefromCollision _geometrycollection true)
  (Physics|AddRadialImpulse _geometrycollection (+ (Transformation|GetWorldLocation _geometrycollection) (* (Math|Vector|GetForwardVector _geometrycollection) 5e+01)) 5.0 (* (/ 1.0 (Class|GameplayStatics|GetGlobalTimeDilation)) 2e+02) "RIF_Constant" true)
  (Physics|SetEnableGravity (Variables|Default|GetGeometryCollection) true)
  (Utilities|FlowControl|Delay 0.2)
  (Actor|DestroyActor))

(fn ConstructionScript)