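; BP_ParkourSpline is a parkour helper actor that supplies start and end points along paired spline edges.
; BeginPlay registers four splines and maps them into two opposite pairs, each spline pointing to its partner.
; FindEndPoint picks the spline nearest the instigator, then writes the closest points on it and its partner into the parkour data as start and end.
; It returns the partner spline.
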(event EventBeginPlay
  (bind _splinemap (Variables|Default|GetSplineMap))
  (Utilities|Array|Add _splinemap (Variables|Default|GetSpline))
  (Utilities|Array|Add _splinemap (Variables|Default|GetSpline1))
  (Utilities|Array|Add _splinemap (Variables|Default|GetSpline2))
  (Utilities|Array|Add _splinemap (Variables|Default|GetSpline3))
  (Utilities|Map|Add (Variables|Default|GetSplineMatchMap) (Variables|Default|GetSpline) (Variables|Default|GetSpline1))
  (Utilities|Map|Add (Variables|Default|GetSplineMatchMap) (Variables|Default|GetSpline1) (Variables|Default|GetSpline))
  (Utilities|Map|Add (Variables|Default|GetSplineMatchMap) (Variables|Default|GetSpline2) (Variables|Default|GetSpline3))
  (Utilities|Map|Add (Variables|Default|GetSplineMatchMap) (Variables|Default|GetSpline3) (Variables|Default|GetSpline2)))

(event Collision|EventActorBeginOverlap
  (params (OtherActor :type Actor%20Object%20Reference)))

(event EventTick
  (params (DeltaSeconds :type Float%20%28single-precision%29)))

(fn ConstructionScript)

(fn FindEndPoint
  (params (Instigator :type Actor%20Object%20Reference) (ParkourDataOut :type S%20Parkour%20Data%20Structure%20%28by%20ref%29))
  (bind _returnvalue (Transformation|GetActorLocation Instigator))
  (bind _returnvalue_2 (Transformation|GetActorLocation Instigator))
  (for (_array_element _array_index) (Variables|Default|GetSplineMap)
    (if (< (Math|Vector|Distance(Vector) (Spline|FindLocationClosesttoWorldLocation _array_element _returnvalue "World") _returnvalue) (LocalVariables|GetCurDistance))
      (LocalVariables|SetIndex _array_index)
      (LocalVariables|SetCurDistance (Math|Vector|Distance(Vector) (Spline|FindLocationClosesttoWorldLocation _array_element _returnvalue "World") _returnvalue))))
  (Utilities|Struct|SetmembersinS_ParkourData ParkourDataOut (Spline|FindLocationClosesttoWorldLocation (Utilities|Array|Get(acopy) (Variables|Default|GetSplineMap) (LocalVariables|GetIndex)) _returnvalue_2 "World") (Spline|FindLocationClosesttoWorldLocation (.Value (Utilities|Map|Find (Variables|Default|GetSplineMatchMap) (Utilities|Array|Get(acopy) (Variables|Default|GetSplineMap) (LocalVariables|GetIndex)))) _returnvalue_2 "World"))
  (return (.Value (Utilities|Map|Find (Variables|Default|GetSplineMatchMap) (Utilities|Array|Get(acopy) (Variables|Default|GetSplineMap) (LocalVariables|GetIndex))))))