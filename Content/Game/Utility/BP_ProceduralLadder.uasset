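; BP_ProceduralLadder is an interactable ladder actor that builds itself from a length and a bar interval.
; The construction script scales both side rails to the length, adds instanced rungs at each interval below the top, and records their heights in an array.
; Interact passes the ladder to BP_PlayerCharacter's TestStartLadder and prints a debug message.
; A getter exposes the rung heights.
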(event EventBeginPlay)

(event Collision|EventActorBeginOverlap
  (params (OtherActor :type Actor%20Object%20Reference)))

(event EventTick
  (params (DeltaSeconds :type Float%20%28single-precision%29)))

(event EventInteract
  (params (InteractingActor :type Actor%20Object%20Reference))
  (bind _asbp_player_character (Utilities|Casting|CastToBP_PlayerCharacter InteractingActor))
  (Default|TestStartLadder _asbp_player_character self)
  (Development|PrintString "Ladder Start"))

(fn ConstructionScript
  (bind _ladderlength (Variables|Ladder|GetLadderLength))
  (bind _returnvalue (/ _ladderlength 1e+02))
  (Utilities|Array|Clear (Variables|Default|GetLadderBarHeightArray))
  (Utilities|FlowControl|Sequence
    (:then_0
      ;[0.15 0.15 0.15 0.5] Ladder Length
      (Transformation|SetWorldScale3D (Variables|Default|Getladder_right) (Math|Vector|MakeVector 0.1 0.1 _returnvalue))
      (Transformation|SetWorldScale3D (Variables|Default|Getladder_left) (Math|Vector|MakeVector 0.1 0.1 _returnvalue)))
    (:then_1
      (for _index (range 1 (Math|Conversions|ToInteger(Byte) (/ (Class|KismetMathLibrary|ToInt64(Float) (Variables|Ladder|GetLadderLength)) (Class|KismetMathLibrary|ToInt64(Float) (Variables|Ladder|GetBarInterval)))))
        (if (> (Variables|Ladder|GetLadderLength) (* _index (Variables|Ladder|GetBarInterval)))
          (Components|InstancedStaticMesh|AddInstance (Variables|Default|GetLadder_Bar) (Math|Transform|MakeTransform (+ (Variables|/Script/Engine.SceneComponent|GetRelativeLocation (Variables|Default|GetLadder_Bar)) (Math|Vector|MakeVector 0.0 0.0 (* _index (Variables|Ladder|GetBarInterval)))) "0, 0, 0" "0.100000,1.000000,0.050000") false)
          (Utilities|Array|Add (Variables|Default|GetLadderBarHeightArray) (* _index (Variables|Ladder|GetBarInterval))))))))

(fn GetLadderBarHeightArray
  (return (Variables|Default|GetLadderBarHeightArray)))