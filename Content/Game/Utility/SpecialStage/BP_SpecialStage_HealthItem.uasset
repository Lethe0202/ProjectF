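; BP_SpecialStage_HealthItem is an interactable health item pickup that returns the player from a special stage.
; Interacting hides the prompt widget, plays a fade-out sequence and runs a timeline in reverse to drive the SphereRadius parameter in MPC_SpecialStageSphre.
; When the timeline finishes, it moves the player to RespawnTransform, plays a fade-in and increments the PFPlayerCharacter health item count.
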(event EventBeginPlay)

(event EventInteract
  (params (InteractingActor :type Actor%20Object%20Reference))
  (Rendering|SetVisibility (Variables|Default|GetWidget) false false)
  (bind _returnvalue (Sequencer|Player|CreateLevelSequencePlayer "/Game/Game/Sequence/Utility/LS_FadeOut.LS_FadeOut" (Utilities|Struct|MakeMovieSceneSequencePlaybackSettings false "(Value=0)" "(TickIntervalSeconds=0.000000,EvaluationBudgetMicroseconds=0.000000,bTickWhenPaused=False,bAllowRounding=True)" 1.0 0.0 false false false false false false "ForceKeepState" false)))
  (Sequencer|Player|Play _returnvalue :!class /Script/MovieScene.MovieSceneSequencePlayer)
  (bind _새_트랙_1 (Timeline|타임라인 ReverseFromEnd)
    (:Update
      (Rendering|Material|SetScalarParameterValue "/Game/Art/Utility/SpecialStage/MPC_SpecialStageSphre.MPC_SpecialStageSphre" "SphereRadius" _새_트랙_1 :!class /Script/Engine.KismetMaterialLibrary))
    (:Finished
      (Transformation|SetActorTransform (Game|GetPlayerCharacter 0) (Variables|Default|GetRespawnTransform))
      (bind _returnvalue_2 (Sequencer|Player|CreateLevelSequencePlayer "/Game/Game/Sequence/Utility/LS_FadeIn.LS_FadeIn" (Utilities|Struct|MakeMovieSceneSequencePlaybackSettings false "(Value=0)" "(TickIntervalSeconds=0.000000,EvaluationBudgetMicroseconds=0.000000,bTickWhenPaused=False,bAllowRounding=True)" 1.0 0.0 false false false false false false "ForceKeepState" false)))
      (Sequencer|Player|Play _returnvalue_2 :!class /Script/MovieScene.MovieSceneSequencePlayer)
      (bind _aspfplayer_character (Utilities|Casting|CastToPFPlayerCharacter (Game|GetPlayerCharacter 0)))
      (Class|PFPlayerCharacter|AddHealthItemCnt _aspfplayer_character 1))))

(event EventVisibleInteractablePrompt
  (params (bVisible :type Boolean))
  (Rendering|SetVisibility (Variables|Default|GetWidget) bVisible false))

(fn ConstructionScript)