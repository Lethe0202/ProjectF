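; BP_BossRommTriggerVolume is a boss room trigger that starts the boss intro and sets up the boss health bar.
; When a player character overlaps its box, it plays the intro level sequence and combat music, then disables the box's collision.
; When the sequence finishes, it adds a boss bar widget to the HUD's top slot, named by the boss's ID.
; Boss health and stamina events update the bars, and zero health removes the widget.
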(event OnComponentBeginOverlap(Box)
  (params (OverlappedComponent :type Primitive%20Component%20Object%20Reference) (OtherActor :type Actor%20Object%20Reference) (OtherComp :type Primitive%20Component%20Object%20Reference) (OtherBodyIndex :type Integer) (bFromSweep :type Boolean) (SweepResult :type Hit%20Result%20Structure%20%28by%20ref%29))
  (Utilities|FlowControl|Sequence
    (:then_0
      (bind _aspfplayer_character (Utilities|Casting|CastToPFPlayerCharacter OtherActor))
      (bind _returnvalue (Sequencer|Player|CreateLevelSequencePlayer (Variables|Default|GetBossIntroSequence)))
      (EventDispatchers|AssignOnFinished _returnvalue (delegate Custom|OnFinished_이벤트))
      (Sequencer|Player|Play _returnvalue :!class /Script/MovieScene.MovieSceneSequencePlayer)
      (Collision|SetCollisionEnabled (Variables|Default|GetBox) "NoCollision")
      (Audio|PlaySound2D "/Game/Art/SFX/BackGround/Fantasy_Starter_Pack/WAVs/The_Adventurer_Combat_Full.The_Adventurer_Combat_Full" 1.0 1.0 0.0 0 0 false))))

(event Custom|OnStaminaChanged_이벤트
  (params (OldValue :type Float%20%28single-precision%29) (NewValue :type Float%20%28single-precision%29) (MaxValue :type Float%20%28single-precision%29) (Instigator :type Actor%20Object%20Reference))
  (Class|ProgressHUDWidget|OnProgressChanged (Variables|/Game/Game/UI/HUD/Combat/WBP_EnemyStatus.WBP_EnemyStatus_C|GetWBP_StaminaBar (Variables|/Game/Game/UI/HUD/Combat/WBP_BossHealthBar.WBP_BossHealthBar_C|GetWBP_EnemyStatus (stale Custom|OnFinished_이벤트 _returnvalue))) OldValue NewValue MaxValue Instigator))

(event Custom|커스텀이벤트
  (params (OldValue :type Float%20%28single-precision%29) (NewValue :type Float%20%28single-precision%29) (MaxValue :type Float%20%28single-precision%29) (Instigator :type Actor%20Object%20Reference))
  (Class|ProgressHUDWidget|OnProgressChanged (Variables|/Game/Game/UI/HUD/Combat/WBP_EnemyStatus.WBP_EnemyStatus_C|GetWBP_HealthBar (Variables|/Game/Game/UI/HUD/Combat/WBP_BossHealthBar.WBP_BossHealthBar_C|GetWBP_EnemyStatus (stale Custom|OnFinished_이벤트 _returnvalue))) OldValue NewValue MaxValue Instigator)
  (if (<= NewValue 0.0)
    (Widget|RemovefromParent (stale Custom|OnFinished_이벤트 _returnvalue))))

(event Custom|OnFinished_이벤트
  (bind _aspfplayer_controller (Utilities|Casting|CastToPFPlayerController (Pawn|GetController (stale OnComponentBeginOverlap(Box) _aspfplayer_character))))
  (bind _returnvalue (UserInterface|CreateWidget "/Game/Game/UI/HUD/Combat/WBP_BossHealthBar.WBP_BossHealthBar_C" _aspfplayer_controller))
  (Class|PFPlayerController|AddWidgettoHUDSlot _aspfplayer_controller "Top" _returnvalue)
  (Utilities|FlowControl|Sequence
    (:then_0
      (bind _aspfcharacter_base (Utilities|Casting|CastToPFCharacterBase (Variables|Default|GetBossActor)))
      (Default|SetDIsplayName _returnvalue (Class|PFCharacterBase|GetID _aspfcharacter_base)))
    (:then_1
      (EventDispatchers|BindEventtoOnHealthStatusChanged (Variables|/Script/ProjectF.PFCharacterBase|GetHealthComponent _aspfcharacter_base) (delegate Custom|커스텀이벤트)))
    (:then_2
      (EventDispatchers|AssignOnStaminaChanged (Variables|/Script/ProjectF.PFCharacterBase|GetStaminaComponent _aspfcharacter_base) (delegate Custom|OnStaminaChanged_이벤트)))))

(event EventBeginPlay)

(event Collision|EventActorBeginOverlap
  (params (OtherActor :type Actor%20Object%20Reference)))

(event EventTick
  (params (DeltaSeconds :type Float%20%28single-precision%29)))

(fn ConstructionScript)